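; PC_Campaign is the campaign player controller that sets up game input and handles pausing.
; On BeginPlay it switches to game-only input and, for the local player, creates a skill system debugger widget fed by the BP_FemalePlayer pawn's skill component.
; The IA_Pause input action passes the pause request to GM_Campaign through its PauseGame call.
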(event `self.ReceiveBeginPlay`
  (`WidgetBlueprintLibrary.SetInputMode_GameOnly` self)
  (if (`self.IsLocalPlayerController`)
    (bind _asbp_female_player (cast `/Game/Characters/BP_FemalePlayer` (`self.K2_GetPawn`)))
    (bind _returnvalue (`|CreateWidget` "/SkillSystem/WBP_SkillSystemDebugger.WBP_SkillSystemDebugger_C" self))
    (`UserWidget.AddToViewport` _returnvalue 0)
    (`/SkillSystem/WBP_SkillSystemDebugger.InitDebugInfo` _returnvalue (`CharacterBase.GetSkillComponent` _asbp_female_player))))

(event `EnhancedInput|/Game/Input/Actions/IA_Pause`
  (params (ActionValue :type Boolean) (ElapsedSeconds :type "Float (double-precision)") (TriggeredSeconds :type "Float (double-precision)") (InputAction :type "InputAction Object Reference" :default "/Game/Input/Actions/IA_Pause.IA_Pause"))
  (:`Triggered`
    (bind _asgm_campaign (cast `/Game/Core/GM_Campaign` (`GameplayStatics.GetGameMode`)))
    (`/Game/Core/GM_Campaign.PauseGame` _asgm_campaign)))

(fn `UserConstructionScript`)