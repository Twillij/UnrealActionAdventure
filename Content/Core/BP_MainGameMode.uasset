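; BP_MainGameMode is the main game mode Blueprint, handling pause and resume through a pause menu widget.
; PauseGame creates WBP_PauseMenu if none exists, adds it to the viewport, switches to UI-only input, shows the cursor and pauses the game.
; ResumeGame removes and clears the stored widget, restores game-only input and unpauses, but leaves the cursor flag unchanged.
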(event `PauseGame`
  (bind _returnvalue (`GameplayStatics.GetPlayerController` 0))
  (`/Engine/EditorBlueprintResources/StandardMacros.IsValid` (`self.PauseMenuWidget`)
    (:`Is Not Valid`
      (bind _returnvalue_2 (`|GenericCreateObject` "/Game/UI/Widgets/WBP_PauseMenu.WBP_PauseMenu_C"))
      (bind _output_get (set `self.PauseMenuWidget` _returnvalue_2))
      (`UserWidget.AddToViewport` _output_get 0)
      (`WidgetBlueprintLibrary.SetInputMode_UIOnlyEx` _returnvalue (`self.PauseMenuWidget`) "DoNotLock" true)
      (set `PlayerController.bShowMouseCursor` true _returnvalue)
      (`GameplayStatics.SetGamePaused` true))))

(event `ResumeGame`
  (`/Engine/EditorBlueprintResources/StandardMacros.IsValid` (`self.PauseMenuWidget`)
    (:`Is Valid`
      (`Widget.RemoveFromParent` (`self.PauseMenuWidget`))
      (set `self.PauseMenuWidget` null)
      (`WidgetBlueprintLibrary.SetInputMode_GameOnly` (`GameplayStatics.GetPlayerController` 0) true)
      (`GameplayStatics.SetGamePaused` false))))

(fn `UserConstructionScript`)